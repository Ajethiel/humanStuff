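; Scannables is a grabbable physics item for motion-controller play that awards its point value to the player pawn when scanned.
; Pickup and Drop toggle physics and attachment, while Scanned passes the points to MotionControllerPawn.
; Kill optionally triggers a delayed explosion that sphere-traces, spawns an emitter and teleports the hit actor to below the origin.
; Gravity, velocity and random-spin logic is left disconnected, with empty stub events.
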(event Custom|Kill
  ;[1 1 1] expire= set the life span of an object in
  (Utilities|FlowControl|Delay 0.2)
  (if (Variables|Default|GetCan_Expolde)
    (CallFunction|Explode)))

(event Custom|Scanned
  ;[1 1 1] Getting points and sending them
  (bind _asmotion_controller_pawn (Utilities|Casting|CastToMotionControllerPawn (Game|Player|GetPlayerPawn 0)))
  (Default|Addingpoints _asmotion_controller_pawn (Variables|Default|GetPointsvalue)))

(event Custom|Grav
  ;[1 1 1] c
)

(event Custom|Explode
  (bind _luigi (Variables|Default|GetLuigi))
  (bind _returnvalue (Transformation|GetWorldLocation _luigi))
  ;[1 1 1] Set explosionon object
  (Utilities|FlowControl|Delay 2.0)
  (bind (_outhit _returnvalue_2) (Collision|SphereTraceByChannel _returnvalue _returnvalue 1e+02 "TraceTypeQuery3" true 0 "None"))
  (if _returnvalue_2
    (Effects|SpawnEmitteratLocation "/Game/StarterContent/Particles/P_Explosion.P_Explosion" (.ImpactPoint (Collision|BreakHitResult _outhit)))
    (Transformation|SetActorLocation (.HitActor (Collision|BreakHitResult _outhit)) "0, 0,-100.000000" false false)))

(event Custom|sET%20gRAV%20ROT
  ;[1 1 1] Rotate
)

(event Custom|Set%20Status%20Qou)

(event EventBeginPlay
  ;[1 1 1] beginplay
  (bind _asshopping_carts (Utilities|Casting|CastToShoppingCarts (Game|Player|GetPlayerPawn 0))))

(event EventPickup
  (params (AttachTo :type Scene%20Component%20Object%20Reference))
  ;[1 1 1] Grab and release
  (Physics|SetSimulatePhysics (Variables|Debug|GetStaticMeshComponent) false)
  (Transformation|AttachComponentToComponent (VehicleSound|GetRootComponent) AttachTo "None" "KeepWorld" "KeepWorld" "KeepWorld" false)
  (Variables|Default|SetGrabbed true)
  (CallFunction|SetStatusQou))

(event EventDrop
  ;[1 1 1] Grab and release
  (Physics|SetSimulatePhysics (Variables|Debug|GetStaticMeshComponent) true)
  (Transformation|DetachFromActor "KeepWorld" "KeepWorld" "KeepWorld")
  (Variables|Default|SetGrabbed false)
  (CallFunction|SetStatusQou))

(fn ConstructionScript
  (Variables|Default|SetDegrees%20per%20sec%20min%20max (Math|Vector2D|MakeVector2D 1.0 2e+01)))