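; BabyCarts is an actor Blueprint for carts that track a distance along a referenced spline.
; Each Tick calls LocationUpdate and then Movement, whose bodies are not shown.
; When Distance comes within a small tolerance of the spline's length, it resets to zero to loop back to the start.
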(event EventBeginPlay
  (|CallParentFunction) ; This node is disabled and will not be called.\nDrag off pins to build functionality.
)

(event Collision|EventActorBeginOverlap
  (params (OtherActor :type Actor%20Object%20Reference)))

(event EventTick
  (params (DeltaSeconds :type Float%20%28single-precision%29))
  (CallFunction|LocationUpdate)
  (CallFunction|Movement)
  (if (Math|Float|NearlyEqual(Float) (Variables|Default|GetDistance) (Spline|GetSplineLength (Variables|/Game/Blueprints/CartSpline.CartSpline_C|GetSpline (Variables|Default|GetSpline))) 1e+01)
    (Variables|Default|SetDistance 0.0)))

(fn ConstructionScript
  (|CallParentFunction))