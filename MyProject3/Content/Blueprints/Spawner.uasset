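; Spawner that moves a sphere from its root toward EndPoint on a timeline, detecting Scannables objects along the way.
; A looping one-second timer sphere-traces at the sphere; each hit spawns a random Scanables class at a random TargetPoint.
; TransferObject then traces between the first two TargetPoints and copies the detected object's points, mesh, lifespan and explode flag onto the Scannables it hits.
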(event Custom|SpawnItem
  (bind _scanables (Variables|Default|GetScanables))
  ;[1 1 1] Teleport objects to specific points
  (bind _outactors (Actor|GetAllActorsOfClass "/Script/Engine.TargetPoint"))
  (Game|SpawnActorfromClass (Utilities|Array|Get(acopy) _scanables (Math|Random|RandomInteger (Utilities|Array|Length _scanables))) (Transformation|GetActorTransform (Utilities|Array|Get(acopy) _outactors (Math|Random|RandomInteger (Utilities|Array|Length _outactors)))) "Undefined" 0 0))

(event Custom|TransferObject
  (params (Pointsvalue :type Float%20%28single-precision%29) (NewMesh :type Static%20Mesh%20Object%20Reference) (LifeSpan :type Float%20%28single-precision%29) (Explode :type Boolean) (NewParam2 :type Boolean) (NewParam3 :type Boolean) (NewParam4 :type Boolean))
  ;[1 1 1] Transfer object points and mesh
  (bind (_outhit _returnvalue) (Collision|SphereTraceByChannel (Transformation|GetActorLocation (Utilities|Array|Get(acopy) (stale Custom|SpawnItem _outactors))) (Transformation|GetActorLocation (Utilities|Array|Get(acopy) (stale Custom|SpawnItem _outactors) 1)) 5e+01 "TraceTypeQuery3" false 0 "ForDuration"))
  (if _returnvalue
    (bind _asscannables (Utilities|Casting|CastToScannables (.HitActor (Collision|BreakHitResult _outhit))))
    (Variables|/Game/Blueprints/Scannables.Scannables_C|SetCan_Expolde _asscannables Explode)
    (Actor|SetLifeSpan _asscannables LifeSpan)
    (Components|StaticMesh|SetStaticMesh (Variables|/Script/Engine.StaticMeshActor|GetStaticMeshComponent _asscannables) NewMesh)
    (bind _output_get (Variables|/Game/Blueprints/Scannables.Scannables_C|SetPointsvalue _asscannables Pointsvalue))
    (Development|PrintString (Utilities|String|ToString(Float) _output_get))))

(event EventBeginPlay
  (Variables|Default|SetSpherelocation (Transformation|GetWorldLocation (Variables|Default|GetDefaultSceneRoot)))
  (Utilities|Time|SetTimerbyFunctionName 0 "Detect" 1.0 true)
  (bind _newtrack_0 (Timeline|Timeline_0 Play)
    (:Update
      (Transformation|SetWorldLocation (Variables|Default|GetSphere) (Math|Vector|Lerp(Vector) (Variables|Default|GetSpherelocation) (Transformation|GetWorldLocation (Variables|Default|GetEnd%20Point)) _newtrack_0) false false))))

(fn ConstructionScript)

(fn Detect
  (bind _sphere (Variables|Default|GetSphere))
  (bind _returnvalue (Transformation|GetWorldLocation _sphere))
  ;[1 1 1] Detecting thespecfics on a object
  (bind (_outhit _returnvalue_2) (Collision|SphereTraceByChannel _returnvalue _returnvalue 5e+01 "TraceTypeQuery3" true 0 "ForDuration"))
  (if _returnvalue_2
    (bind _asscannables (Utilities|Casting|CastToScannables (.HitActor (Collision|BreakHitResult _outhit))))
    (CallFunction|SpawnItem)
    (CallFunction|TransferObject (Variables|/Game/Blueprints/Scannables.Scannables_C|GetPointsvalue _asscannables) (Variables|/Script/Engine.StaticMeshComponent|GetStaticMesh (Variables|/Script/Engine.StaticMeshActor|GetStaticMeshComponent _asscannables)) (Actor|GetLifeSpan _asscannables) (Variables|/Game/Blueprints/Scannables.Scannables_C|GetCan_Expolde _asscannables) false false false)))