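; SpawnNumeroDos is a spawner that periodically creates copies of the actors held in its Items array.
; A looping timer started on BeginPlay calls SpawnItem every few seconds, spawning one actor of each entry's class at the spawner's location with random rotation.
; The lookup that would fill Items with all Scannables actors is disconnected, so this graph never populates the array.
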(event Custom|SpawnItem
  (for (_array_element _array_index) (Variables|Default|GetItems)
    (Game|SpawnActorfromClass (Utilities|GetClass _array_element) (Math|Transform|MakeTransform (Transformation|GetActorLocation) (Math|Random|RandomRotator false) "1,1,1") "Undefined" 0 0)))

(event EventBeginPlay
  (Utilities|Time|SetTimerbyFunctionName 0 "SpawnItem" 3.0 true))

(fn ConstructionScript)