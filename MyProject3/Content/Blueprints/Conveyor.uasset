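; Conveyor actor that pushes Scannables entering its Box trigger, ignoring the entry if the item is grabbed.
; A random roll usually shifts overlapping items along the conveyor's forward by editable Speed.
; Other rolls first disable the entering item's gravity and set its Velocity along either its own or the conveyor's forward, then offset items by it.
; Movement repeats through Delay nodes looping back to re-query the overlaps, rather than using Tick.
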(event OnComponentBeginOverlap(Box)
  (params (OverlappedComponent :type Primitive%20Component%20Object%20Reference) (OtherActor :type Actor%20Object%20Reference) (OtherComp :type Primitive%20Component%20Object%20Reference) (OtherBodyIndex :type Integer) (bFromSweep :type Boolean) (SweepResult :type Hit%20Result%20Structure%20%28by%20ref%29))
  (bind _asscannables (Utilities|Casting|CastToScannables OtherActor))
  (if (not (Variables|/Game/Blueprints/Scannables.Scannables_C|GetGrabbed _asscannables))
    (switch int (Math|Random|RandomIntegerinRange 0 4)
      (:0
        (for _array_element (Collision|GetOverlappingActors (Variables|Default|GetBox) "/Game/Blueprints/Scannables.Scannables_C" :!class /Script/Engine.PrimitiveComponent) :!label _label
          (Transformation|AddActorWorldOffset _array_element (* (Math|Vector|GetForwardVector (Transformation|GetActorRotation)) (* (Variables|Default|GetSpeed) 1.0)))
          (Utilities|FlowControl|Delay 0.1)
          ;[1 1 1] Pushes Forward
          (Utilities|FlowControl|Delay 0.1)
          (goto _label)))
      (:1
        (Default|SETGRAVROT _asscannables)
        (Physics|SetEnableGravity (Variables|/Script/Engine.StaticMeshActor|GetStaticMeshComponent _asscannables) false)
        (Variables|/Game/Blueprints/Scannables.Scannables_C|SetCurrent _asscannables false)
        (Variables|/Game/Blueprints/Scannables.Scannables_C|SetVelocity _asscannables "0, 0, 0")
        (bind _output_get (Variables|/Game/Blueprints/Scannables.Scannables_C|SetVelocity _asscannables (* (Math|Vector|GetForwardVector (Transformation|GetActorRotation _asscannables)) (Variables|Default|GetSpeed))))
        (for _array_element_2 (Collision|GetOverlappingActors (Variables|Default|GetBox) "/Game/Blueprints/Scannables.Scannables_C" :!class /Script/Engine.PrimitiveComponent) :!label _label_2
          (Transformation|AddActorWorldOffset _array_element_2 _output_get)
          (Utilities|FlowControl|Delay 0.1)
          (Utilities|FlowControl|Delay 0.1)
          (goto _label_2)))
      (:2
        (Default|SETGRAVROT _asscannables)
        (Physics|SetEnableGravity (Variables|/Script/Engine.StaticMeshActor|GetStaticMeshComponent _asscannables) false)
        (Variables|/Game/Blueprints/Scannables.Scannables_C|SetCurrent _asscannables false)
        (Variables|/Game/Blueprints/Scannables.Scannables_C|SetVelocity _asscannables "0, 0, 0")
        (bind _output_get_2 (Variables|/Game/Blueprints/Scannables.Scannables_C|SetVelocity _asscannables (* (Math|Vector|GetForwardVector (Transformation|GetActorRotation)) (Variables|Default|GetSpeed))))
        (for _array_element_3 (Collision|GetOverlappingActors (Variables|Default|GetBox) "/Game/Blueprints/Scannables.Scannables_C" :!class /Script/Engine.PrimitiveComponent) :!label _label_3
          (Transformation|AddActorWorldOffset _array_element_3 _output_get_2)
          (Utilities|FlowControl|Delay 0.2)
          (Utilities|FlowControl|Delay 0.1)
          (goto _label_3)))
      (:3
        (goto _label))
      (:4
        (goto _label)))))

(fn ConstructionScript)