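; CartSpawn is a spawner Blueprint meant to periodically create shopping carts at its own transform.
; BeginPlay starts a looping timer targeting "SapwnCart", a misspelling that does not match the SpawnCart event.
; SpawnCart prints a debug message and spawns a cart without any count check.
; The cart-limit check and the AI move to each cart's CartPoint are disconnected and never run.
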(event Custom|SpawnCart
  ;[1 1 1] Check for cart amount and spawns another
  (Development|PrintString "Hello")
  (bind _returnvalue (Game|SpawnActorfromClass "/Game/Blueprints/ShoppingCarts.ShoppingCarts_C" (Math|Transform|MakeTransform (Transformation|GetActorLocation) (Transformation|GetActorRotation) "1,1,1") "Undefined" 0 0)))

(event EventBeginPlay
  (Utilities|Time|SetTimerbyFunctionName 0 "SapwnCart" 2.0 true))

(fn ConstructionScript)