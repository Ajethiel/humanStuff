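; Shopping cart pawn that wanders the level and collects scanned Scannables items tagged with its color.
; A looping timer calls Move, which sends it by AI MoveTo to a random navigable point nearby and plays a rattle sound.
; Box overlaps add matching items' points until the cart reaches its target, then it emits sparks and destroys itself.
; Disconnected timeline and rotation experiments remain unused.
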(event OnComponentBeginOverlap(Box)
  (params (OverlappedComponent :type Primitive%20Component%20Object%20Reference) (OtherActor :type Actor%20Object%20Reference) (OtherComp :type Primitive%20Component%20Object%20Reference) (OtherBodyIndex :type Integer) (bFromSweep :type Boolean) (SweepResult :type Hit%20Result%20Structure%20%28by%20ref%29))
  ;[1 1 1] Point Check
  (bind _asscannables (Utilities|Casting|CastToScannables OtherActor))
  (if (and (Variables|/Game/Blueprints/Scannables.Scannables_C|GetIsScanned _asscannables) (Actor|ActorHasTag OtherActor (Variables|Color|GetColor)))
    (Development|PrintString "MMMM TASTY!")
    (bind _output_get (Variables|Default|SetPoints (+ (Variables|/Game/Blueprints/Scannables.Scannables_C|GetPointsvalue _asscannables) (Variables|Default|GetPoints))))
    (Development|PrintString (Utilities|String|ToString(Float) _output_get))
    (Default|Scanned _asscannables)
    (if (>= _output_get (Variables|Default|GetPointsNeeded))
      (Effects|SpawnEmitteratLocation "/Game/StarterContent/Particles/P_Sparks.P_Sparks" (Transformation|GetActorLocation) (Transformation|GetActorRotation))
      (Actor|DestroyActor)
      (Development|PrintString "Aw fuck"))
    (else
      (Development|PrintString "I aint no theif"))))

(event Custom|Move
  (bind _returnvalue (Transformation|GetActorLocation))
  (bind _area (Variables|Movement|GetArea))
  (bind _randomlocation (Class|NavigationSystemV1|GetRandomPointinNavigableRadius _returnvalue _area 0 0))
  ;[1 1 1] Move
  (Utilities|FlowControl|DoOnce false :!label _label
    (:Completed
      (AI|AIMoveTo self _randomlocation 0 5.0 false
        (:then
          (Variables|Movement|SetDest _randomlocation)
          (Audio|PlaySoundatLocation "/Game/Audio/se_cartRattle.se_cartRattle" (Transformation|GetActorLocation) "0, 0, 0" 1.0 1.0 0.0 0 0 0)
          (goto _label Reset))))))

(event Custom|Back)

(event EventTick
  (params (DeltaSeconds :type Float%20%28single-precision%29)))

(event EventBeginPlay
  (bind _floatingpawnmovement (Variables|Default|GetFloatingPawnMovement))
  ;[1 1 1] Move tha cart and pause for a moment
  ;[1 1 1] Colors
  (Utilities|FlowControl|Sequence
    (:then_0
      ;;[1 1 1] Controls speed
      (Variables|/Script/Engine.FloatingPawnMovement|SetMaxSpeed _floatingpawnmovement (Variables|Movement|GetSpeed))
      (Variables|/Script/Engine.FloatingPawnMovement|SetAcceleration _floatingpawnmovement (Variables|Movement|GetAccel))
      (Utilities|Time|SetTimerbyFunctionName 0 "Move" (Variables|Movement|GetTime) true))
    (:then_1
      (Rendering|Material|SetMaterial (Variables|Default|GetStaticMesh) 0 (Variables|Color|GetColor2)))))

(fn ConstructionScript)